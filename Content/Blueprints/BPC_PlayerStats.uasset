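; Player stats component that tracks health and stamina for BP_ThirdPersonCharacter and displays them on its HUD.
; BeginPlay caches the owning character, whose HUDWidget is written to directly.
; Change functions apply deltas with clamping, and the max-value variants shift the current value by the same amount.
; Health and stamina changes update their progress bars, while max health changes refresh only the text and max stamina changes leave the HUD untouched.
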(event EventBeginPlay
  (bind _asbp_third_person_character (Utilities|Casting|CastToBP_ThirdPersonCharacter (Components|GetOwner)))
  (Variables|Default|SetPlayer%20Character _asbp_third_person_character))

(fn ChangeMaxHealth
  (params (Value :type Integer))
  (Variables|Health|SetMaxHealth (+ Value (Variables|Health|GetMaxHealth)))
  (bind _output_get (Variables|Health|SetCurrent%20Health (+ Value (Variables|Health|GetCurrent%20Health))))
  (if (< _output_get 0)
    (Variables|Health|SetCurrent%20Health 0)
    (elif (> (Variables|Health|GetCurrent%20Health) (Variables|Health|GetMaxHealth))
      (Variables|Health|SetCurrent%20Health (Variables|Health|GetMaxHealth))))
  (Health|SetHealthText))

(fn ChangeHealth
  (params (Value :type Integer))
  (bind _output_get (Variables|Health|SetCurrent%20Health (+ Value (Variables|Health|GetCurrent%20Health))))
  (if (> _output_get (Variables|Health|GetMaxHealth))
    (Variables|Health|SetCurrent%20Health (Variables|Health|GetMaxHealth))
    (elif (<= (Variables|Health|GetCurrent%20Health) 0)
      (Variables|Health|SetCurrent%20Health 0)))
  (Health|SetHealthProgressBar)
  (Health|SetHealthText))

(fn ChangeStamina
  (params (Value :type Integer))
  (bind _output_get (Variables|Stamina|SetCurrentStamina (+ Value (Variables|Stamina|GetCurrentStamina))))
  (if (> _output_get (Variables|Stamina|GetMaxStamina))
    (Variables|Stamina|SetCurrentStamina (Variables|Stamina|GetMaxStamina))
    (elif (< (Variables|Stamina|GetCurrentStamina) 0)
      (Variables|Stamina|SetCurrentStamina 0)))
  (Stamina|SetStaminaProgressBar))

(fn ChangeMaxStamina
  (params (Value :type Integer))
  (Variables|Stamina|SetMaxStamina (+ Value (Variables|Stamina|GetMaxStamina)))
  (bind _output_get (Variables|Stamina|SetCurrentStamina (+ Value (Variables|Stamina|GetCurrentStamina))))
  (if (< _output_get 0)
    (Variables|Stamina|SetCurrentStamina 0)
    (elif (> (Variables|Stamina|GetCurrentStamina) (Variables|Stamina|GetMaxStamina))
      (Variables|Stamina|SetCurrentStamina (Variables|Stamina|GetMaxStamina)))))

(fn SetHealthProgressBar
  (Progress|SetPercent (Variables|/Game/UI/WB_HUD.WB_HUD_C|GetHealthProgressBar (Variables|/Game/ThirdPerson/Blueprints/BP_ThirdPersonCharacter.BP_ThirdPersonCharacter_C|GetHUD%20Widget (Variables|Default|GetPlayer%20Character))) (/ (Math|Conversions|ToFloat(Integer) (Variables|Health|GetCurrent%20Health)) (Math|Conversions|ToFloat(Integer) (Variables|Health|GetMaxHealth)))))

(fn SetStaminaProgressBar
  (Progress|SetPercent (Variables|/Game/UI/WB_HUD.WB_HUD_C|GetStaminaProgressBar (Variables|/Game/ThirdPerson/Blueprints/BP_ThirdPersonCharacter.BP_ThirdPersonCharacter_C|GetHUD%20Widget (Variables|Default|GetPlayer%20Character))) (Math|Conversions|ToFloat(Integer) (/ (Variables|Stamina|GetCurrentStamina) (Variables|Stamina|GetMaxStamina)))))

(fn SetHealthText
  (Rendering|Components|TextRender|SetText (Variables|/Game/UI/WB_HUD.WB_HUD_C|GetHealthAmountText (Variables|/Game/ThirdPerson/Blueprints/BP_ThirdPersonCharacter.BP_ThirdPersonCharacter_C|GetHUD%20Widget (Variables|Default|GetPlayer%20Character))) (Utilities|Text|FormatText "{Health}/{Max Health}" (Variables|Health|GetCurrent%20Health) (Variables|Health|GetMaxHealth))))